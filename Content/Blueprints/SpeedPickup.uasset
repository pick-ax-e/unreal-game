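; SpeedPickup is a pickup Blueprint that boosts the player's speed when collected.
; It overrides On pickup, calls the parent implementation, then runs Give Player Speed.
; That function casts player pawn 0 to TopDownCharacter, multiplies its Speed variable by a large fixed factor, destroys the pickup and prints a confirmation.
; The file contains no timer or reset for the boost, and its event graph is inactive.
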(fn `Give Player Speed`
  (bind _astop_down_character (cast `/Game/Blueprints/TopDownCharacter` (`GameplayStatics.GetPlayerPawn` 0)))
  (set `/Game/Blueprints/TopDownCharacter.Speed` (* (`/Game/Blueprints/TopDownCharacter.Speed` _astop_down_character) 50.0) _astop_down_character)
  (`self.K2_DestroyActor`)
  (`KismetSystemLibrary.PrintString` "Speed Given"))

(fn `On pickup`
  (`parent.On pickup`)
  (`self.Give Player Speed`))

(fn `UserConstructionScript`
  (`parent.UserConstructionScript`))